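; Base Blueprint for area-target active abilities in the turn-based strategy template that use a custom target pattern.
; SpawnCustomTargetArea only returns the CustomTargetPattern reference.
; A separate event spawns hex-mesh static mesh actors at supplied locations.
; Disconnected nodes that would read tile offsets from the pattern data table and spawn hexes rotated by actor yaw never run.
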(event Custom|SpawnTilesAtLoacations
  (params (TileLocations :type Array%20of%20Vectors))
  (for _array_element TileLocations
    (bind _returnvalue (Game|SpawnActorfromClass "/Script/Engine.StaticMeshActor" (Math|Transform|MakeTransform _array_element "0, 0, 0" "1.000000,1.000000,1.000000") "AlwaysSpawn" "MultiplyWithRoot" 0 0))
    (Components|StaticMesh|SetStaticMesh (Variables|/Script/Engine.StaticMeshActor|GetStaticMeshComponent _returnvalue) "/Game/TurnBasedStrategyRPGTemplate/Meshes/SM_HexMesh.SM_HexMesh")))

(fn ConstructionScript
  (|CallParentFunction))

(fn SpawnCustomTargetArea
  (return (Variables|Default|GetCustomTargetPattern)))